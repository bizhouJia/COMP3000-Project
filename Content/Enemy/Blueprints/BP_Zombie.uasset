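; BP_Zombie is a side-scrolling 2D flipbook enemy that chases and attacks the BP_MC player.
; Tick moves it along X toward the player inside ViewCollision, flipping it and switching idle, run and attack flipbooks.
; AttackCollision starts a delayed loop damaging the player until they leave or die.
; CE_BeAttacked reduces HP; Tick detects death only while viewing, then plays death flipbooks and destroys the actor.
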(event OnComponentBeginOverlap(ViewCollision)
  (params (OverlappedComponent :type Primitive%20Component%20Object%20Reference) (OtherActor :type Actor%20Object%20Reference) (OtherComp :type Primitive%20Component%20Object%20Reference) (OtherBodyIndex :type Integer) (bFromSweep :type Boolean) (SweepResult :type Hit%20Result%20Structure%20%28by%20ref%29))
  ;[1 1 1] Handle Attack
  (Utilities|Casting|CastToBP_MC OtherActor)
  (Variables|Default|SetViewing true))

(event OnComponentEndOverlap(ViewCollision)
  (params (OverlappedComponent :type Primitive%20Component%20Object%20Reference) (OtherActor :type Actor%20Object%20Reference) (OtherComp :type Primitive%20Component%20Object%20Reference) (OtherBodyIndex :type Integer))
  ;[1 1 1] Handle Attack
  (Utilities|Casting|CastToBP_MC OtherActor)
  (Variables|Default|SetViewing false))

(event OnComponentBeginOverlap(AttackCollision)
  (params (OverlappedComponent :type Primitive%20Component%20Object%20Reference) (OtherActor :type Actor%20Object%20Reference) (OtherComp :type Primitive%20Component%20Object%20Reference) (OtherBodyIndex :type Integer) (bFromSweep :type Boolean) (SweepResult :type Hit%20Result%20Structure%20%28by%20ref%29))
  ;[1 1 1] Handle Attack
  (bind _asbp_mc (Utilities|Casting|CastToBP_MC OtherActor))
  (Variables|Default|SetAttackCharacter _asbp_mc)
  (Variables|Default|SetCanAttack true)
  (Variables|Default|SetAttacking true)
  (Utilities|FlowControl|Delay 0.7 :!label _label)
  (if (Variables|Default|GetCanAttack)
    (Default|CEbeAttacked (Variables|Default|GetAttackCharacter) (Variables|Default|GetATK))
    (if (> (Variables|/Game/Characters/MC/Blueprints/BP_MC.BP_MC_C|GetHP (Variables|Default|GetAttackCharacter)) 0.0)
      (goto _label)
      (else
        (Variables|Default|SetCanAttack false))))
  (Variables|Default|SetAttacking false))

(event OnComponentEndOverlap(AttackCollision)
  (params (OverlappedComponent :type Primitive%20Component%20Object%20Reference) (OtherActor :type Actor%20Object%20Reference) (OtherComp :type Primitive%20Component%20Object%20Reference) (OtherBodyIndex :type Integer))
  ;[1 1 1] Handle Attack
  (Utilities|Casting|CastToBP_MC OtherActor)
  (Variables|Default|SetCanAttack false))

(event Custom|UpdateAnimation
  ;[1 1 1] Handle Animation
  (Sprite|SetFlipbook (Variables|Default|GetSprite) (select (> (Math|Vector|VectorLength (Transformation|GetVelocity)) 0.0) "/Game/Enemy/Animation/Run_Ani_Z.Run_Ani_Z" "/Game/Enemy/Animation/Idle_Ani_Z.Idle_Ani_Z")))

(event Custom|CE_BeAttacked
  (params (Damage :type Float%20%28double-precision%29))
  ;[1 1 1] Handle Hurt
  (Variables|Default|SetHP (- (Variables|Default|GetHP) Damage)))

(event Custom|CE_Attack
  ;[1 1 1] Handle Animation
  (Sprite|SetFlipbook (Variables|Default|GetSprite) "/Game/Enemy/Animation/Attack_Ani_Z.Attack_Ani_Z")
  (Components|Movement|StopMovementImmediately (Variables|Character|GetCharacterMovement)))

(event EventBeginPlay
  (Class|ActorComponent|SetIsReplicated (Variables|Default|GetSprite) true))

(event Collision|EventActorBeginOverlap
  (params (OtherActor :type Actor%20Object%20Reference)))

(event EventTick
  (params (DeltaSeconds :type Float%20%28single-precision%29))
  ;[1 1 1] Tick-Updates animation
  (if (Variables|Default|GetIsDead)
    (Utilities|FlowControl|DoOnce false
      (:Completed
        (Sprite|SetFlipbook (Variables|Default|GetSprite) "/Game/Enemy/Animation/Dead_Ani_Z.Dead_Ani_Z")
        (Utilities|FlowControl|Delay 0.6)
        (Sprite|SetFlipbook (Variables|Default|GetSprite) "/Game/Enemy/Animation/DeadLoop_Ani_Z.DeadLoop_Ani_Z")
        (Utilities|FlowControl|Delay 0.5)
        (Actor|DestroyActor)))
    (else
      (if (Variables|Default|GetViewing)
        (bind _asbp_mc (Utilities|Casting|CastToBP_MC (Game|GetPlayerCharacter 0)))
        (if (>= (- (.X (Math|Vector|BreakVector (Transformation|GetActorLocation _asbp_mc))) (.x (Transformation|GetActorLocation))) 0.0)
          (Variables|Default|SetBisMovingRight true)
          (else
            (Variables|Default|SetBisMovingRight false)))
        (Pawn|Input|AddMovementInput "1.000000,0.000000,0.000000" (- (.X (Math|Vector|BreakVector (Transformation|GetActorLocation _asbp_mc))) (.x (Transformation|GetActorLocation))) false)
        (if (Variables|Default|GetAttacking)
          (CallFunction|CEAttack)
          (else
            (CallFunction|UpdateAnimation :!label _label)
            (Math|Float|CompareFloat (.X (Math|Vector|BreakVector (Variables|/Script/Engine.MovementComponent|GetVelocity (Pawn|GetMovementComponent)))) 0.0
              (:>
                (Transformation|SetActorRotation "0, 0, 0" :!label _label_2))
              (:==
                (if (Variables|Default|GetBisMovingRight)
                  (goto _label_2)
                  (else
                    (Transformation|SetActorRotation "0.000000,180.000000,0.000000" :!label _label_3))))
              (:<
                (goto _label_3)))))
        (else
          (goto _label)))
      (if (<= (Variables|Default|GetHP) 0.0)
        (Variables|Default|SetIsDead true)))))

(event Input|AxisEvents|InputAxisMoveRight
  (params (AxisValue :type Float%20%28single-precision%29))
  ;[1 1 1] Handle Movement
  (if (> AxisValue 0.0)
    (Variables|Default|SetBisMovingRight true)
    (elif (< AxisValue 0.0)
      (Variables|Default|SetBisMovingRight false)))
  (Pawn|Input|AddMovementInput "1.000000,0.000000,0.000000" AxisValue false))

(fn ConstructionScript)